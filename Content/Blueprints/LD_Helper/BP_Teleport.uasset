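; BP_Teleport is a level-design helper actor that teleports BP_Player both ways between two triggers, landing slightly above the other with its rotation.
; A shared cooldown and per-trigger occupancy flags guard against immediate bounce-back.
; The construction script places both triggers and two spline points from LocationA and LocationB.
; BeginPlay draws a long-lived debug line linking the triggers.
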(event OnComponentBeginOverlap(TriggerA)
  (params (OverlappedComponent :type Primitive%20Component%20Object%20Reference) (OtherActor :type Actor%20Object%20Reference) (OtherComp :type Primitive%20Component%20Object%20Reference) (OtherBodyIndex :type Integer) (bFromSweep :type Boolean) (SweepResult :type Hit%20Result%20Structure%20%28by%20ref%29))
  (bind _triggerb (Variables|Default|GetTriggerB))
  (bind _asbp_player (Utilities|Casting|CastToBP_Player OtherActor))
  (if (and (Variables|Default|GetCanTp) (not (Variables|Default|GetIsInB)))
    (Variables|Default|SetCanTp false)
    (Variables|Default|SetIsInA true)
    (Transformation|Teleport _asbp_player (+ (Transformation|GetWorldLocation _triggerb) "0.000000,0.000000,70.000000") (Transformation|GetWorldRotation _triggerb))
    (Utilities|FlowControl|Delay (Variables|Default|GetTpCooldown))
    (Variables|Default|SetCanTp true)))

(event OnComponentEndOverlap(TriggerA)
  (params (OverlappedComponent :type Primitive%20Component%20Object%20Reference) (OtherActor :type Actor%20Object%20Reference) (OtherComp :type Primitive%20Component%20Object%20Reference) (OtherBodyIndex :type Integer))
  (Utilities|Casting|CastToBP_Player OtherActor)
  (Variables|Default|SetIsInA false))

(event OnComponentBeginOverlap(TriggerB)
  (params (OverlappedComponent :type Primitive%20Component%20Object%20Reference) (OtherActor :type Actor%20Object%20Reference) (OtherComp :type Primitive%20Component%20Object%20Reference) (OtherBodyIndex :type Integer) (bFromSweep :type Boolean) (SweepResult :type Hit%20Result%20Structure%20%28by%20ref%29))
  (bind _triggera (Variables|Default|GetTriggerA))
  (bind _asbp_player (Utilities|Casting|CastToBP_Player OtherActor))
  (if (and (Variables|Default|GetCanTp) (not (Variables|Default|GetIsInA)))
    (Variables|Default|SetCanTp false)
    (Variables|Default|SetIsInB true)
    (Transformation|Teleport _asbp_player (+ (Transformation|GetWorldLocation _triggera) "0.000000,0.000000,70.000000") (Transformation|GetWorldRotation _triggera))
    (Utilities|FlowControl|Delay (Variables|Default|GetTpCooldown))
    (Variables|Default|SetCanTp true)))

(event OnComponentEndOverlap(TriggerB)
  (params (OverlappedComponent :type Primitive%20Component%20Object%20Reference) (OtherActor :type Actor%20Object%20Reference) (OtherComp :type Primitive%20Component%20Object%20Reference) (OtherBodyIndex :type Integer))
  (Utilities|Casting|CastToBP_Player OtherActor)
  (Variables|Default|SetIsInB false))

(event EventBeginPlay
  (Rendering|Debug|DrawDebugLine (Transformation|GetWorldLocation (Variables|Default|GetTriggerA)) (Transformation|GetWorldLocation (Variables|Default|GetTriggerB)) "(R=1.000000,G=1.000000,B=1.000000,A=1.000000)" 3.6e+03 1.0))

(fn ConstructionScript
  (bind _spline (Variables|Default|GetSpline))
  (Spline|SetLocationatSplinePoint _spline 0 (Variables|Default|GetLocationA) "Local" true)
  (Spline|SetLocationatSplinePoint _spline 1 (Variables|Default|GetLocationB) "Local" true)
  (Transformation|SetRelativeLocation (Variables|Default|GetTriggerA) (Variables|Default|GetLocationA) false false)
  (Transformation|SetRelativeLocation (Variables|Default|GetTriggerB) (Variables|Default|GetLocationB) false false))