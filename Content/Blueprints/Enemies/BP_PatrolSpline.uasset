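; BP_PatrolSpline is a patrol route that supplies world-space destinations from the points of a spline.
; GetNextDest advances the current point index and returns its location, while GetCurrentDest returns the location without advancing.
; Looping mode wraps the index with a hard-coded modulo of four rather than the spline's point count.
; Non-looping mode ping-pongs by flipping Direction at either end of the spline.
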(fn ConstructionScript)

(fn GetNextDest
  (params (IsLooping :type Boolean))
  (if IsLooping
    (Variables|Default|SetCurrentSplinePoint (Math|Integer|%(Integer) (+ (Variables|Default|GetCurrentSplinePoint) 1) 4))
    (else
      (if (or (< (+ (Variables|Default|GetCurrentSplinePoint) (Variables|Default|GetDirection)) 0) (>= (+ (Variables|Default|GetCurrentSplinePoint) (Variables|Default|GetDirection)) (Spline|GetNumberOfSplinePoints (Variables|Default|GetSpline))))
        (Variables|Default|SetDirection (* (Variables|Default|GetDirection) -1)))
      (Variables|Default|SetCurrentSplinePoint (+ (Variables|Default|GetCurrentSplinePoint) (Variables|Default|GetDirection)))))
  (return (Spline|GetLocationatSplinePoint (Variables|Default|GetSpline) (Variables|Default|GetCurrentSplinePoint) "World")))

(fn GetCurrentDest
  (return (Spline|GetLocationatSplinePoint (Variables|Default|GetSpline) (Variables|Default|GetCurrentSplinePoint) "World")))