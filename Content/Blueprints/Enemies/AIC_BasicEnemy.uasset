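; AI controller for BP_Enemy that walks the possessed enemy along its assigned patrol spline.
; On possess it starts a move loop, requesting the next spline point (looping or not per the enemy's setting) and pausing briefly on arrival.
; A failed move retries the current point once; a second failure prints an error, draws a debug sphere at that location, then moves on.
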(event Custom|StartNextMoveTo
  (bind _enemyref (Variables|Default|GetEnemyRef))
  (bind _nextpointlocation (Default|GetNextDest (Variables|/Game/Blueprints/Enemies/BP_Enemy.BP_Enemy_C|GetPatrolSpline _enemyref) (Variables|/Game/Blueprints/Enemies/BP_Enemy.BP_Enemy_C|GetIsLoopingPatrol _enemyref)))
  (AI|AIMoveTo _enemyref _nextpointlocation 0 2e+01 false
    (:OnSuccess
      (Utilities|FlowControl|Delay 2.0)
      (CallFunction|StartNextMoveto))
    (:OnFail
      (CallFunction|TryAgainReachCurrentPoint))))

(event Custom|TryAgainReachCurrentPoint
  (bind _enemyref (Variables|Default|GetEnemyRef))
  (bind _currentpointlocation (Default|GetCurrentDest (Variables|/Game/Blueprints/Enemies/BP_Enemy.BP_Enemy_C|GetPatrolSpline _enemyref)))
  (AI|AIMoveTo _enemyref _currentpointlocation 0 2e+01 false
    (:OnSuccess
      _)
    (:OnFail
      (Development|PrintString (Utilities|String|ToString(Text) (Utilities|Text|FormatText "Error: BP_Enemy: A point spline looks unreachable or Enemy is blocked. Please check location: {locX} {LocY}, {LocZ}" (.X (Math|Vector|BreakVector _currentpointlocation)) (.Y (Math|Vector|BreakVector _currentpointlocation)) (.Z (Math|Vector|BreakVector _currentpointlocation)))) true true "(R=1.000000,G=0.000000,B=0.000000,A=1.000000)" 3e+01)
      (Rendering|Debug|DrawDebugSphere _currentpointlocation 25.0 12 "(R=1.000000,G=0.000000,B=0.000000,A=1.000000)" 3e+01 2.0)))
  (CallFunction|StartNextMoveto))

(event EventPossess
  (params (PossessedPawn :type Pawn%20Object%20Reference))
  (bind _asbp_enemy (Utilities|Casting|CastToBP_Enemy PossessedPawn))
  (bind _output_get (Variables|Default|SetEnemyRef _asbp_enemy))
  (Utilities|IsValid (Variables|/Game/Blueprints/Enemies/BP_Enemy.BP_Enemy_C|GetPatrolSpline _output_get)
    (:Is%20Valid
      (Utilities|FlowControl|Delay 0.0)
      (CallFunction|StartNextMoveto))))

(fn ConstructionScript)